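; Rumor actor for the main world: a tentacled Niagara character that wakes on click or touch, plays a voice line, then toggles between talking and silent.
; Timelines animate tentacle growth and rotation, while baked Constant-Q audio analysis at playback time drives its mouth.
; Talking retracts opinions and shrinks anemones; silence or audio end restores them.
; HTTP handlers spawn anemones from JSON categories, but their requests are disconnected.
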(event OnClicked(Sphere)
  (params (TouchedComponent :type Primitive%20Component%20Object%20Reference) (ButtonPressed :type Key%20Structure :default "None"))
  ;[1 1 1] Not neccisary, just to debug, so we can check with onclick function
  ;;[1 1 1] Wake up Rumor, set niagara tenticles  to 600 from point
  (Niagara|SetNiagaraVariable(Float) (Variables|Default|GetRumor) "BPCallbackHandlerPointForce" 6e+02)
  ;;[1 1 1] check if animation just played, restet when game goes in sleepmode
  (if (Variables|Default|GetsleepMode)
    (Utilities|FlowControl|Delay 1.0)
    (Variables|Default|SetsleepMode false))
  ;;[1 1 1] check if audio is playing, play sound if not and keep reference, stop sound
  (if (Variables|Default|GetaudioIsPlaying)
    (Components|Activation|SetActive (stale _returnvalue) false true)
    (Variables|Default|SetaudioIsPlaying false)
    (else
      (bind _returnvalue (Audio|SpawnSound2D "/Game/Sound/rumor_test.rumor_test" 1.0 1.0 0.0 0))
      (Variables|Default|SetaudioIsPlaying true))))

(event Custom|playbackChange
  (params (PlayingSoundWave :type Sound%20Wave%20Object%20Reference) (PlaybackPercent :type Float%20%28single-precision%29))
  ;[1 1 1] begin settings
  ;;[1 1 1] set  intro audio to play and play talking animation
  (Variables|Default|SetPlayedTime (* PlaybackPercent (Variables|Default|GetDurationAudio)))
  (for _array_element (Class|ConstantQNRT|GetNormalizedChannelConstantQatTime (Variables|Default|GetConstantRef) (Variables|Default|GetPlayedTime))
    (Niagara|SetNiagaraVariable(Float) (Variables|Default|GetRumor) "rumorMouth" (+ (* _array_element 5e+01) 7e+01))))

(event Custom|onCategoriesComplete
  (params (Status :type Byte) (ResponseString :type String))
  ;[1 1 1] getData
  (bind _returnvalue (Class|HTTPRequestClient|ResponseStringtoJSON ResponseString))
  (bind _returnvalue_2 (Class|HTTPRequestClient|GetStringArrayfromJSONObject _returnvalue "categories"))
  (for _array_element _returnvalue_2
    (Utilities|FlowControl|Sequence
      (:then_0
        (Development|PrintString _array_element))
      (:then_1
        (bind _returnvalue_3 (Class|HTTPRequestClient|GetObjectArrayfromJSONObject (stale Custom|OnHTTPRequestComplete _returnvalue) _array_element))
        (for (_array_element_2 _array_index) _returnvalue_3
          (bind _returnvalue_4 (Class|HTTPRequestClient|GetStringfromJSONObject _array_element_2 "text"))
          (Utilities|FlowControl|Sequence
            (:then_0
              (bind _outrownames (DataTable|GetDataTableRowNames "/Game/structures/anemonePositionData.anemonePositionData")))
            (:then_1
              (bind _returnvalue_5 (Utilities|GetDataTableRow "/Game/structures/anemonePositionData.anemonePositionData" (Utilities|Array|Get(acopy) _outrownames _array_index))))
            (:then_2
              (bind _returnvalue_6 (Game|SpawnActorfromClass "/Game/bluePrints/BP_annemoon.BP_annemoon_C" (Math|Transform|MakeTransform (Math|Vector|MakeVector (Math|Conversions|ToFloat(Integer) (Math|Random|RandomIntegerinRange 570 1080)) (Math|Conversions|ToFloat(Integer) (Math|Random|RandomIntegerinRange -610 710)) (Math|Conversions|ToFloat(Integer) (Math|Random|RandomIntegerinRange -1150 -1150)))) "Undefined" 0 (Utilities|Text|ToText(String) _array_element) (Utilities|Text|ToText(String) _returnvalue_4) 0))
              (Rendering|Components|TextRender|SetText (Variables|/Game/bluePrints/BP_annemoon.BP_annemoon_C|GetTextRender _returnvalue_6) (Utilities|Text|ToText(String) _array_element))
              (Default|StartGrow _returnvalue_6))))))))

(event Custom|rumor%20shut%20up
  ;[1 1 1] shut up
  (Variables|Default|Setrumor%20talk true)
  (Utilities|FlowControl|Sequence
    (:then_0
      (CallFunction|ShakeOut))
    (:then_1
      (Utilities|FlowControl|Delay 0.05)
      (Utilities|FlowControl|Sequence
        (:then_0
          (bind _outactors (Actor|GetAllActorsOfClass "/Game/bluePrints/BP_annemoon.BP_annemoon_C"))
          (for _array_element _outactors
            (Default|StartGrow _array_element)))
        (:then_1
          (bind _outactors_2 (Actor|GetAllActorsOfClass "/Game/bluePrints/BP_opinion.BP_opinion_C"))
          (for _array_element_2 _outactors_2
            (Default|ShootOpinions _array_element_2)))
        (:then_2
          (Niagara|SetNiagaraVariable(Float) (Variables|Default|GetRumor) "rumorMouth" 75.0))))
    (:then_2
      (Audio|Components|Audio|Stop (Variables|Default|GetrumorVoice)))
    (:then_3
      (bind _outactors_3 (Actor|GetAllActorsOfClass "/Game/bluePrints/BP_opinion_Child_Highlighted.BP_opinion_Child_Highlighted_C"))
      (for _array_element_3 _outactors_3
        (Default|ActivateHighlight _array_element_3)))))

(event Custom|OnHTTPRequestComplete
  (params (Status :type Byte) (ResponseString :type String))
  ;[1 1 1] getData
  (bind _returnvalue (Class|HTTPRequestClient|ResponseStringtoJSON ResponseString))
  (bind _returnvalue_2 (Class|HTTPRequestClient|GetObjectArrayfromJSONObject _returnvalue (stale Custom|onCategoriesComplete _array_element)))
  (for (_array_element _array_index) _returnvalue_2
    (bind _returnvalue_3 (Class|HTTPRequestClient|GetStringfromJSONObject _array_element "text"))
    (Utilities|FlowControl|Sequence
      (:then_0
        (bind _outrownames (DataTable|GetDataTableRowNames "/Game/structures/anemonePositionData.anemonePositionData")))
      (:then_1
        (bind _returnvalue_4 (Utilities|GetDataTableRow "/Game/structures/anemonePositionData.anemonePositionData" (Utilities|Array|Get(acopy) _outrownames _array_index))))
      (:then_2
        (bind _returnvalue_5 (Game|SpawnActorfromClass "/Game/bluePrints/BP_annemoon.BP_annemoon_C" (Math|Transform|MakeTransform (Math|Vector|MakeVector (Math|Conversions|ToFloat(Integer) (Math|Random|RandomIntegerinRange 570 1080)) (Math|Conversions|ToFloat(Integer) (Math|Random|RandomIntegerinRange -610 710)) (Math|Conversions|ToFloat(Integer) (Math|Random|RandomIntegerinRange -1150 -1150)))) "Undefined" 0 (Utilities|Text|ToText(String) (stale Custom|onCategoriesComplete _array_element)) (Utilities|Text|ToText(String) _returnvalue_3) 0))
        (Rendering|Components|TextRender|SetText (Variables|/Game/bluePrints/BP_annemoon.BP_annemoon_C|GetTextRender _returnvalue_5) (Utilities|Text|ToText(String) (stale Custom|onCategoriesComplete _array_element)))
        (Default|StartGrow _returnvalue_5)))))

(event Custom|OnAudioFinished_Event_0
  ;[1 1 1] animation after talking
  (Utilities|FlowControl|Sequence
    (:then_0
      (Utilities|FlowControl|DoOnce false
        (:Completed
          (Variables|Default|SetfirstPlayDone true))))
    (:then_1
      (CallFunction|RumorShutUp))))

(event Custom|rumor%20start%20talking
  ;[1 1 1] start talking actions
  (Variables|Default|Setrumor%20talk false)
  (Utilities|FlowControl|Sequence
    (:then_0
      (bind _outactors (Actor|GetAllActorsOfClass "/Game/bluePrints/BP_opinion.BP_opinion_C"))
      (for _array_element _outactors
        (Default|RetractOpinions _array_element)
        (Default|StopGlow _array_element)))
    (:then_1
      (CallFunction|Shakein))
    (:then_2
      (Utilities|FlowControl|Delay 0.2)
      (Audio|Components|Audio|Play (Variables|Default|GetrumorVoice) 0.0))
    (:then_3
      (Viewport|RemoveAllWidgets))
    (:then_4
      (bind _outactors_2 (Actor|GetAllActorsOfClass "/Game/bluePrints/BP_annemoon.BP_annemoon_C"))
      (for _array_element_2 _outactors_2
        (Rendering|Components|TextRender|SetTextRenderColor (Variables|/Game/bluePrints/BP_annemoon.BP_annemoon_C|GetTextRender _array_element_2) (Variables|Default|Getoriginal%20color%20text%20annemoon))))
    (:then_5
      (bind _outactors_3 (Actor|GetAllActorsOfClass "/Game/bluePrints/BP_annemoon.BP_annemoon_C"))
      (for _array_element_3 _outactors_3
        (Default|Shrink _array_element_3)))
    (:then_6
      (bind _outactors_4 (Actor|GetAllActorsOfClass "/Game/bluePrints/BP_opinion_Child_Highlighted.BP_opinion_Child_Highlighted_C"))
      (for _array_element_4 _outactors_4
        (Default|DeactivateHighlight _array_element_4)))))

(event Custom|shake%20in
  ;[1 1 1] shake animation
  (bind _newtrack_0 (Timeline|shake Reverse)
    (:Update
      (Transformation|SetActorRotation (Math|Rotator|MakeRotator 0.0 0.0 (Math|Float|Lerp 0.0 -1e+01 _newtrack_0))))))

(event Custom|shake%20out
  ;[1 1 1] shake animation
  (bind _newtrack_0 (Timeline|shake PlayFromStart)
    (:Update
      (Transformation|SetActorRotation (Math|Rotator|MakeRotator 0.0 0.0 (Math|Float|Lerp 0.0 -1e+01 _newtrack_0))))))

(event EventBeginPlay
  ;[1 1 1] begin settings
  (Utilities|FlowControl|Sequence
    (:then_0
      ;;[1 1 1] Set niagara tenticles length and drag
      (Niagara|SetNiagaraVariable(Float) (Variables|Default|GetRumor) "BPCallbackHandlerPointForce" 2e+02)
      (Niagara|SetNiagaraVariable(Float) (Variables|Default|GetRumor) "dragTentacles" 15.0))
    (:then_1
      ;;[1 1 1] set  intro audio to play and play talking animation
      (Audio|Components|Audio|SetSound (Variables|Default|GetrumorVoice) (Variables|Default|GetSound))
      (Variables|Default|SetDurationAudio (Variables|/Script/Engine.SoundBase|GetDuration (Variables|Default|GetSound)))
      (EventDispatchers|BindEventtoOnAudioPlaybackPercent (Variables|Default|GetrumorVoice) (delegate Custom|playbackChange)))))

(event Collision|EventActorBeginOverlap
  (params (OtherActor :type Actor%20Object%20Reference)))

(event MouseInput|EventActorOnClicked
  (params (ButtonPressed :type Key%20Structure :default "None"))
  ;[1 1 1] click event
  (if (Variables|Default|Getwake%20up%20rumor)
    ;;[1 1 1] Wake up rumor
    (Utilities|FlowControl|Sequence
      (:then_0
        ;;;[1 1 1] Set niagara tenticles  to 600 from point
        (bind _newtrack_2 (Timeline|growTentacles PlayFromStart)
          (:Update
            (Niagara|SetNiagaraVariable(Float) (Variables|Default|GetRumor) "BPCallbackHandlerPointForce" (Math|Float|Lerp 2e+02 6e+02 _newtrack_2)))))
      (:then_1
        ;;;[1 1 1] set length tentacles
        (Niagara|SetNiagaraVariable(Float) (Variables|Default|GetRumor) "dragTentacles" 3.5))
      (:then_2
        (Utilities|FlowControl|Delay 1.2)
        (Audio|Components|Audio|Play (Variables|Default|GetrumorVoice) 0.0))
      (:then_3
        (bind _returnvalue (Actor|GetActorOfClass "/Game/bluePrints/BP_splineFollower.BP_splineFollower_C"))
        (Default|MoveObject _returnvalue))
      (:then_4
        (Variables|Default|Setwake%20up%20rumor false)))
    (elif (Variables|Default|GetfirstPlayDone)
      (if (Variables|Default|Getrumor%20talk)
        (CallFunction|RumorStartTalking)
        (else
          (CallFunction|RumorShutUp))))))

(event EventTick
  (params (DeltaSeconds :type Float%20%28single-precision%29))
  ;[1 1 1] animation after talking
  (EventDispatchers|AssignOnAudioFinished (Variables|Default|GetrumorVoice) (delegate Custom|OnAudioFinished_Event_0)))

(event EventActorOnInputTouchBegin
  (params (FingerIndex :type ETouchIndex%20Enum :default "Touch1"))
  ;[1 1 1] click event
  (if (Variables|Default|Getwake%20up%20rumor)
    ;;[1 1 1] Wake up rumor
    (Utilities|FlowControl|Sequence
      (:then_0
        ;;;[1 1 1] Set niagara tenticles  to 600 from point
        (bind _newtrack_2 (Timeline|growTentacles PlayFromStart)
          (:Update
            (Niagara|SetNiagaraVariable(Float) (Variables|Default|GetRumor) "BPCallbackHandlerPointForce" (Math|Float|Lerp 2e+02 6e+02 _newtrack_2)))))
      (:then_1
        ;;;[1 1 1] set length tentacles
        (Niagara|SetNiagaraVariable(Float) (Variables|Default|GetRumor) "dragTentacles" 3.5))
      (:then_2
        (Utilities|FlowControl|Delay 1.2)
        (Audio|Components|Audio|Play (Variables|Default|GetrumorVoice) 0.0))
      (:then_3
        (bind _returnvalue (Actor|GetActorOfClass "/Game/bluePrints/BP_splineFollower.BP_splineFollower_C"))
        (Default|MoveObject _returnvalue))
      (:then_4
        (Variables|Default|Setwake%20up%20rumor false)))
    (elif (Variables|Default|GetfirstPlayDone)
      (if (Variables|Default|Getrumor%20talk)
        (CallFunction|RumorStartTalking)
        (else
          (CallFunction|RumorShutUp))))))

(fn ConstructionScript)