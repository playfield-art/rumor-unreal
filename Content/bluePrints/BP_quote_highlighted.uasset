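; BP_quote_highlighted is a quote actor variant that extends its parent's quote behavior with a highlight driven by the Pulse0 component.
; Spawning a new quote runs the parent logic, then activates the pulse after a short delay, while summoning a quote runs the parent logic and deactivates it.
; Separate activateHighlight and deactivateHighlight events also switch the pulse on and off directly.
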(event Custom|activateHighlight
  (Components|Activation|Activate (Variables|Default|Getpulse_0) false))

(event Custom|deactivateHighlight
  (Components|Activation|Deactivate (Variables|Default|Getpulse_0)))

(event EventBeginPlay
  (|CallParentFunction) ; This node is disabled and will not be called.\nDrag off pins to build functionality.
)

(event Collision|EventActorBeginOverlap
  (params (OtherActor :type Actor%20Object%20Reference))
  (|CallParentFunction OtherActor) ; This node is disabled and will not be called.\nDrag off pins to build functionality.
)

(event EventSummonQuote
  (|CallParentFunction)
  (Components|Activation|Deactivate (Variables|Default|Getpulse_0)))

(event EventSpawnNewQuote
  (|CallParentFunction)
  (Utilities|FlowControl|Delay 0.5)
  (Components|Activation|Activate (Variables|Default|Getpulse_0) false))

(fn ConstructionScript
  (|CallParentFunction))