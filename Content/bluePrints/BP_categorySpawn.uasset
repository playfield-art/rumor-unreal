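; Spawner actor that binds to BP_MainWorld's category-creation event on BeginPlay and creates BP_category actors from JSON quote data.
; CreateCategory parses each entry's title, overall summary, tags and statistics, passing only the last statistic read to the spawned actor.
; Actors spawn with slight random XY jitter around the position for the category index and show the event's UITitle.
; The StartGrow call is disconnected.
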(event Custom|CreateCategory
  (params (quoteData :type Array%20of%20JSON%20Object%20Structures) (UITitle :type String) (categoryIndex :type Integer))
  (for _array_element quoteData
    (Utilities|FlowControl|Sequence
      (:then_0
        (bind _returnvalue (Class|HTTPRequestClient|GetObjectfromJSONObject _array_element "summary"))
        (bind _returnvalue_2 (Class|HTTPRequestClient|GetObjectfromJSONObject _returnvalue "overall")))
      (:then_1
        (bind _returnvalue_3 (Class|HTTPRequestClient|GetObjectfromJSONObject _array_element "meta"))
        (bind _returnvalue_4 (Class|HTTPRequestClient|GetStringArrayfromJSONObject _returnvalue_3 "tags")))
      (:then_2
        (bind _returnvalue_5 (Class|HTTPRequestClient|GetObjectArrayfromJSONObject _returnvalue_3 "statistics"))
        (for _array_element_2 _returnvalue_5
          (bind _returnvalue_6 (Class|HTTPRequestClient|GetStringfromJSONObject _array_element_2 "value"))
          (bind _returnvalue_7 (Class|HTTPRequestClient|GetStringfromJSONObject _array_element_2 "name"))))
      (:then_3
        (bind _returnvalue_8 (Class|HTTPRequestClient|GetObjectfromJSONObject _array_element "title")))
      (:then_4
        (bind _returnvalue_9 (Game|SpawnActorfromClass "/Game/bluePrints/BP_category.BP_category_C" (Math|Transform|MakeTransform (+ (Math|Vector|MakeVector (Math|Conversions|ToFloat(Integer) (+ (Math|Random|RandomIntegerinRange -10 10) 0)) (Math|Conversions|ToFloat(Integer) (+ (Math|Random|RandomIntegerinRange -10 10) 0)) (Math|Conversions|ToFloat(Integer) (Math|Random|RandomIntegerinRange 0 0))) (Utilities|Array|Get(acopy) (Variables|Default|GetCategoryPositions) categoryIndex))) "AdjustIfPossibleButAlwaysSpawn" 0 _returnvalue_8 _returnvalue_2 _returnvalue_7 (Math|Conversions|ToFloat(Integer) _returnvalue_6) _returnvalue_4 0))
        (Rendering|Components|TextRender|SetText (Variables|/Game/bluePrints/BP_category.BP_category_C|GetTextRender _returnvalue_9) (Utilities|Text|ToText(String) UITitle))))))

(event EventBeginPlay
  (bind _outactors (Actor|GetAllActorsOfClass "/Game/bluePrints/BP_MainWorld.BP_MainWorld_C"))
  (EventDispatchers|BindEventtoCreateCategories (Utilities|Array|Get(acopy) _outactors) (delegate Custom|CreateCategory)))

(fn ConstructionScript)