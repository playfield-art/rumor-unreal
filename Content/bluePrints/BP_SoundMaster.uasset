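; BP_SoundMaster is an audio visualizer actor that plays a sound and scales a sphere from its spectral data.
; On BeginPlay it starts playback and binds to the playback-percent callback, converting percent to seconds using the sound's duration.
; That time samples channel 0 of normalized Constant-Q data from ConstantRef.
; Each band value sets the same sphere's scale in turn, so only the last band remains visible.
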(event Custom|playbackChange
  (params (PlayingSoundWave :type Sound%20Wave%20Object%20Reference) (PlaybackPercent :type Float%20%28single-precision%29))
  (Variables|Default|SetPlayedTime (* PlaybackPercent (Variables|Default|GetDuration)))
  (for _array_element (Class|ConstantQNRT|GetNormalizedChannelConstantQatTime (Variables|Default|GetConstantRef) (Variables|Default|GetPlayedTime))
    (Transformation|SetWorldScale3D (Variables|Default|GetSphere) (* _array_element 1e+01))))

(event EventBeginPlay
  (Audio|Components|Audio|SetSound (Variables|Default|GetAudio) (Variables|Default|GetSound))
  (Variables|Default|SetDuration (Variables|/Script/Engine.SoundBase|GetDuration (Variables|Default|GetSound)))
  (EventDispatchers|BindEventtoOnAudioPlaybackPercent (Variables|Default|GetAudio) (delegate Custom|playbackChange))
  (Audio|Components|Audio|Play (Variables|Default|GetAudio) 0.0))

(event Collision|EventActorBeginOverlap
  (params (OtherActor :type Actor%20Object%20Reference)))

(event EventTick
  (params (DeltaSeconds :type Float%20%28single-precision%29)))

(fn ConstructionScript)