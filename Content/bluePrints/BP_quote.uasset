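; Clickable opinion sphere that spawns out of the BP_MainWorld Rumor, orbits a center, and reveals a localized quote when summoned.
; Click or touch moves it before the camera via timelines, fading materials and text, while language switcher items are disabled; background or repeat clicks retract it.
; Tick sine-bobs the summoned sphere while still rotating its saved orbit position for the return.
; Empty Niagara events are left for child Blueprints.
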(event OnClicked(Sphere)
  (params (TouchedComponent :type Primitive%20Component%20Object%20Reference) (ButtonPressed :type Key%20Structure :default "None"))
  ;[1 1 1] click opinion
  (if (not (Variables|Default|GetisAnimating))
    (if (Variables|Default|GetisSummoned)
      (CallFunction|RetracktQuote)
      (else
        (CallFunction|SummonQuote)))))

(event OnInputTouchBegin(Sphere)
  (params (FingerIndex :type ETouchIndex%20Enum :default "Touch1") (TouchedComponent :type Primitive%20Component%20Object%20Reference))
  ;[1 1 1] click opinion
  (if (not (Variables|Default|GetisAnimating))
    (if (Variables|Default|GetisSummoned)
      (CallFunction|RetracktQuote)
      (else
        (CallFunction|SummonQuote)))))

(event OnClicked(bg)
  (params (TouchedComponent :type Primitive%20Component%20Object%20Reference) (ButtonPressed :type Key%20Structure :default "None"))
  ;[1 1 1] Retrackt opinion on bg click/touch
  (if (Variables|Default|GetisSummoned)
    (CallFunction|RetracktQuote)))

(event OnInputTouchBegin(bg)
  (params (FingerIndex :type ETouchIndex%20Enum :default "Touch1") (TouchedComponent :type Primitive%20Component%20Object%20Reference))
  ;[1 1 1] Retrackt opinion on bg click/touch
  (if (Variables|Default|GetisSummoned)
    (CallFunction|RetracktQuote)))

(event Custom|startGlow
  ;[1 1 1] glow animation control
  (Components|Activation|Activate (Variables|Default|Getglow) false))

(event Custom|stopGlow
  ;[1 1 1] glow animation control
  (Components|Activation|Deactivate (Variables|Default|Getglow)))

(event Custom|retracktQuote
  ;[1 1 1] animation when opinion needs to go back to mothership
  (Utilities|FlowControl|Sequence
    (:then_0
      (CallFunction|HideText))
    (:then_1
      (CallFunction|MaterialtoOpaque))
    (:then_2
      (Components|Activation|Deactivate (Variables|Default|GetFX_swirl)))
    (:then_3
      (Utilities|FlowControl|Delay 1.6)
      (CallFunction|BacktoPlace))
    (:then_4
      (bind _foundwidgets (Widget|GetAllWidgetsOfClass "/Game/UIElements/W_LanguageSwitcherItem.W_LanguageSwitcherItem_C" false))
      (for _array_element _foundwidgets
        (Widget|SetIsEnabled _array_element true)))))

(event Custom|summonQuote
  ;[1 1 1] summon actions
  (Utilities|FlowControl|Sequence
    (:then_0
      (CallFunction|SetTextOfOpinion))
    (:then_1
      (CallFunction|MoveQuotetoFrontOfCamera))
    (:then_2
      ;;[1 1 1] deactivate glow after delay
      (Utilities|FlowControl|Delay 0.2)
      (CallFunction|StopGlow))
    (:then_3
      (Utilities|FlowControl|Delay 0.5)
      (Components|Activation|Activate (Variables|Default|GetFX_swirl) false))
    (:then_4
      (bind _foundwidgets (Widget|GetAllWidgetsOfClass "/Game/UIElements/W_LanguageSwitcherItem.W_LanguageSwitcherItem_C" false))
      (for _array_element _foundwidgets
        (Widget|SetIsEnabled _array_element false)))))

(event Custom|deactivateNiagara
  ;[1 1 1] used in child bp
)

(event Custom|moveQuoteToFrontOfCamera
  ;[1 1 1] animation opinion goes from current location to location in front of camera
  (Variables|Default|SetisAnimating true)
  (Variables|Default|SetpreviousLocation (Transformation|GetActorLocation))
  (CallFunction|DeactivateHighlight)
  (bind (_direction _positioncurve _displacecurve) (Timeline|Timeline_2 PlayFromStart)
    (:Update
      (CallFunction|AnimatetoFrontOfCamera _displacecurve (Variables|Default|GetsummonedScale) _positioncurve (Variables|Default|GetsummonedPosition)))
    (:Finished
      (CallFunction|SetMaterials)
      (Variables|Default|SetisAnimating false))))

(event Custom|setMaterials
  ;[1 1 1] summon actions
  (Variables|Default|SetisSummoned true)
  (CallFunction|MaterialtoTransparent)
  (CallFunction|ShowText))

(event Custom|MaterialToTransparent
  ;[1 1 1] materialLogic
  (Utilities|FlowControl|Sequence
    (:then_0
      (bind _materialopacity (Timeline|materialChange PlayFromStart)
        (:Update
          (Rendering|Material|SetScalarParameterValueonMaterials (Variables|Default|GetSphere) "opacity" _materialopacity))))
    (:then_1
      (bind _materialopacity_2 (Timeline|Timeline_1 ReverseFromEnd)
        (:Update
          (Rendering|Material|SetScalarParameterValueonMaterials (Variables|Default|Getbg) "bgOpacity" (* _materialopacity_2 0.8)))))))

(event Custom|MaterialToOpaque
  ;[1 1 1] materialLogic
  (Rendering|Material|SetScalarParameterValueonMaterials (Variables|Default|Getbg) "bgOpacity" 0.0)
  (bind _materialopacity (Timeline|materialChange ReverseFromEnd)
    (:Update
      (Rendering|Material|SetScalarParameterValueonMaterials (Variables|Default|GetSphere) "opacity" _materialopacity))))

(event Custom|shootOpinions
  ;[1 1 1] shoot /retract opinions animation
  (Utilities|FlowControl|Sequence
    (:then_0
      ;;[1 1 1] set animation for opinions from center location to random location given by BP_opinionSpawn
      (bind _track (Timeline|Timeline_0 PlayFromStart)
        (:Update
          (bind _rumorlocation (CallFunction|GetRumorLocation))
          (Transformation|SetActorTransform (Math|Transform|MakeTransform (Math|Vector|Lerp(Vector) _rumorlocation (Variables|Default|GetinitialLocation) _track) "0, 0, 0" (Math|Vector|Lerp(Vector) "0, 0, 0" (Variables|Default|GetinitialScale) _track))))))
    (:then_1
      (CallFunction|ActivateNiagara))))

(event Custom|retractOpinions
  ;[1 1 1] shoot /retract opinions animation
  (Utilities|FlowControl|Sequence
    (:then_0
      ;;[1 1 1] set animation for opinions from center location to random location given by BP_opinionSpawn
      (bind _track (Timeline|Timeline_0 ReverseFromEnd)
        (:Update
          (bind _rumorlocation (CallFunction|GetRumorLocation))
          (Transformation|SetActorTransform (Math|Transform|MakeTransform (Math|Vector|Lerp(Vector) _rumorlocation (Variables|Default|GetinitialLocation) _track) "0, 0, 0" (Math|Vector|Lerp(Vector) "0, 0, 0" (Variables|Default|GetinitialScale) _track))))))
    (:then_1
      (CallFunction|DeactivateNiagara))))

(event Custom|hideText
  ;[1 1 1] animation to reveal inside text
  (bind _textopacity (Timeline|textOpacityTimelineReverse PlayFromStart)
    (:Update
      (Rendering|Material|SetScalarParameterValue (Variables|Default|GettextMaterial) "textOpacity" _textopacity :!class /Script/Engine.MaterialInstanceDynamic))))

(event Custom|spawn%20new%20quote
  ;[1 1 1] spawn new actor after delay from rumor  to space
  (bind _returnvalue (Actor|GetActorOfClass "/Game/bluePrints/BP_MainWorld.BP_MainWorld_C"))
  (if (not (Variables|/Game/bluePrints/BP_MainWorld.BP_MainWorld_C|GetaudioIsPlaying _returnvalue))
    (bind _track (Timeline|SpawnTimeline PlayFromStart)
      (:Update
        (bind _rumorlocation (CallFunction|GetRumorLocation))
        (Transformation|SetActorTransform (Math|Transform|MakeTransform (Math|Vector|Lerp(Vector) _rumorlocation (Variables|Default|GetinitialLocation) _track) "0, 0, 0" (Math|Vector|Lerp(Vector) "0, 0, 0" (Variables|Default|GetinitialScale) _track)))))))

(event Custom|activateHighlight
  (Components|Activation|Activate (Variables|Default|Getpulse) false))

(event Custom|showText
  ;[1 1 1] animation to reveal inside text
  (bind _textopacity (Timeline|textOpacityTimeline PlayFromStart)
    (:Update
      (Rendering|Material|SetScalarParameterValue (Variables|Default|GettextMaterial) "textOpacity" _textopacity :!class /Script/Engine.MaterialInstanceDynamic))))

(event Custom|activateNiagara
  ;[1 1 1] used in child bp
)

(event Custom|back%20to%20place
  ;[1 1 1] back to place
  (Variables|Default|SetisAnimating true)
  (bind _newtrack_0 (Timeline|backToPositionAnimationTimeline PlayFromStart)
    (:Update
      (Transformation|SetActorTransform (Math|Transform|MakeTransform (Math|Vector|Lerp(Vector) (Transformation|GetActorLocation) (Variables|Default|GetpreviousLocation) _newtrack_0) "0, 0, 0" (Math|Vector|Lerp(Vector) (Transformation|GetActorScale3D) (Variables|Default|GetinitialScale) _newtrack_0))))
    (:Finished
      (Variables|Default|SetisSummoned false)
      (Variables|Default|SettotalTime 0.0)
      (Variables|Default|SetisAnimating false))))

(event Custom|deactivateHighlight
  (Components|Activation|Deactivate (Variables|Default|Getpulse)))

(event EventBeginPlay
  (bind _bg (Variables|Default|Getbg))
  ;[1 1 1] begin settings
  (Utilities|FlowControl|Sequence
    (:then_0
      (Rendering|Components|TextRender|SetWorldSize (Variables|Default|GetopinionText) 0.0)
      (Variables|Default|SetinitialLocation (Transformation|GetActorLocation))
      (Variables|Default|SetinitialScale (Transformation|GetActorScale3D)))
    (:then_1
      ;;[1 1 1] set opinions out of sight in the beginning so it can spawn out of rumor
      (Transformation|SetActorLocation "-1000000.000000, 0, 0" false false))
    (:then_2
      (CallFunction|RandomizeRotationMesh (Variables|Default|GetSphere)))
    (:then_3
      (CallFunction|SetDynamicMaterials (Variables|Default|GetSphere) _bg _bg (Variables|Default|GetopinionText))
      (Rendering|Material|SetScalarParameterValue (Variables|Default|GettextMaterial) "textOpacity" 0.0 :!class /Script/Engine.MaterialInstanceDynamic))
    (:then_4
      (Rendering|Components|TextRender|SetWorldSize (Variables|Default|GetopinionText) (Variables|Default|GetquoteTextScale)))))

(event EventTick
  (params (DeltaSeconds :type Float%20%28single-precision%29))
  ;[1 1 1] rotate opinions around the x=0 y=0 z=0 axis
  (if (Variables|Default|GetisSummoned)
    (Utilities|FlowControl|Sequence
      (:then_0
        ;[1 1 1] move quote
        (bind _displacementvector (CallFunction|CreateDisplacementVector DeltaSeconds))
        (Transformation|SetActorLocation (+ _displacementvector (Variables|Default|GetsummonedPosition)) false false))
      (:then_1
        (bind _returnvalue (CallFunction|CalculatePositionAfterRotation (Variables|Default|GetpreviousLocation) DeltaSeconds))
        (Variables|Default|SetpreviousLocation _returnvalue)))
    (else
      (bind _returnvalue_2 (CallFunction|CalculatePositionAfterRotation (Transformation|GetActorLocation) DeltaSeconds))
      (Transformation|SetActorLocation _returnvalue_2 false false))))

(fn ConstructionScript)

(fn CreateDisplacementVector
  (bind _output_get (Variables|Default|SettotalTime (+ 0.0 (Variables|Default|GettotalTime))))
  (return (Math|Vector|MakeVector (Math|Trig|Sin(Radians) (* (+ _output_get 14.0) 0.2)) (Math|Trig|Sin(Radians) (* (+ _output_get 3.0) 0.3)) (Math|Trig|Sin(Radians) (* (+ _output_get 2.0) 0.1)))))

(fn CalculatePositionAfterRotation
  (params (InVect :type Vector) (A :type Float%20%28double-precision%29))
  (return (+ (Math|Vector|RotateVectorAroundAxis InVect (* A (Variables|Default|GetSpeed)) (Variables|Default|GetAxis)) (Variables|Default|GetCenter%20Location))))

(fn CreateDisplacementVector
  (params (DeltaSeconds :type Float%20%28double-precision%29))
  (bind _output_get (Variables|Default|SettotalTime (+ DeltaSeconds (Variables|Default|GettotalTime))))
  (return (* (Math|Vector|MakeVector (Math|Trig|Sin(Radians) (* (+ _output_get 0.0) 0.8)) (Math|Trig|Sin(Radians) (* (+ _output_get 0.0) 0.9)) (Math|Trig|Sin(Radians) (* (+ _output_get 0.0) 0.5))) (Variables|Default|GetmovementQuote))))

(fn RandomizeRotationMesh
  (params (self2 :type Scene%20Component%20Object%20Reference))
  (Transformation|SetWorldRotation self2 (Math|Rotator|MakeRotator 0.0 0.0 (Math|Float|MapRangeClamped (Math|Random|RandomFloat) 0.0 1.0 0.0 3.6e+02)) false false))

(fn SetDynamicMaterials
  (params (sphere :type Primitive%20Component%20Object%20Reference) (bg :type Primitive%20Component%20Object%20Reference) (bgMesh :type Mesh%20Component%20Object%20Reference) (Text :type Primitive%20Component%20Object%20Reference))
  (Rendering|Material|CreateDynamicMaterialInstance sphere 0 "/Game/materials/waterColor_Inst.waterColor_Inst" "None" :!class /Script/Engine.PrimitiveComponent)
  (Rendering|Material|CreateDynamicMaterialInstance bg 0 "/Game/materials/bg_quotes.bg_quotes" "None" :!class /Script/Engine.PrimitiveComponent)
  (Rendering|Material|SetScalarParameterValueonMaterials bgMesh "bgOpacity" 0.0)
  (bind _returnvalue (Rendering|Material|CreateDynamicMaterialInstance Text 0 "/Game/materials/quoteTextMaterial.quoteTextMaterial" "None" :!class /Script/Engine.PrimitiveComponent))
  (Variables|Default|SettextMaterial _returnvalue))

(fn AnimatetoFrontOfCamera
  (params (DisplaceCurve :type Vector) (SummonedScale :type Vector) (Alpha :type Float%20%28single-precision%29) (SummonedPosition :type Vector))
  (Transformation|SetActorTransform (Math|Transform|MakeTransform (Math|Vector|Lerp(Vector) (+ (Transformation|GetActorLocation) (* DisplaceCurve "0.000000,2.000000,4.000000")) SummonedPosition Alpha) "0, 0, 0" (Math|Vector|Lerp(Vector) (Transformation|GetActorScale3D) SummonedScale Alpha))))

(fn SetTextOfOpinion
  (bind _returnvalue (Class|HTTPRequestClient|GetStringfromJSONObject (Variables|Default|Getquote) (Class|KismetInternationalizationLibrary|GetCurrentLanguage)))
  (Rendering|Components|TextRender|SetText (Variables|Default|GetopinionText) (Utilities|Text|ToText(String) _returnvalue)))

(fn GetRumorLocation
  (bind _returnvalue (Actor|GetActorOfClass "/Game/bluePrints/BP_MainWorld.BP_MainWorld_C"))
  (return (Transformation|GetWorldLocation (Variables|/Game/bluePrints/BP_MainWorld.BP_MainWorld_C|GetRumor _returnvalue))))