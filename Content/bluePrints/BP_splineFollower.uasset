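; BP_splineFollower is an actor that travels along the spline of a BP_splinepath actor.
; BeginPlay caches the path found by GetActorOfClass; movement starts only when the MoveObject event is called.
; MoveObject plays a timeline at a rate of one over TimeToCompleteInSeconds.
; Each update lerps distance over the spline length and sets the actor transform, sampling location in world space but rotation in local space.
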(event Custom|Move%20Object
  (bind _spline_ref (Variables|Default|Getspline%20REF))
  (bind _spline (Variables|/Game/bluePrints/BP_splinepath.BP_splinepath_C|GetSpline _spline_ref))
  (Components|Timeline|SetPlayRate (Variables|Default|GetMove%20Object%20T) (/ 1.0 (Variables|Default|Gettime%20to%20complete%20%28in%20seconds%29)))
  (bind _move_track (Timeline|Move%20Object%20T Play)
    (:Update
      (Transformation|SetActorTransform (Math|Transform|MakeTransform (Spline|GetLocationatDistanceAlongSpline _spline (Math|Float|Lerp 0.0 (Spline|GetSplineLength (Variables|/Game/bluePrints/BP_splinepath.BP_splinepath_C|GetSpline (Variables|Default|Getspline%20REF))) _move_track) "World") (Spline|GetRotationatDistanceAlongSpline _spline (Math|Float|Lerp 0.0 (Spline|GetSplineLength (Variables|/Game/bluePrints/BP_splinepath.BP_splinepath_C|GetSpline (Variables|Default|Getspline%20REF))) _move_track) "Local") "1.000000,1.000000,1.000000")))))

(event EventBeginPlay
  (bind _returnvalue (Actor|GetActorOfClass "/Game/bluePrints/BP_splinepath.BP_splinepath_C"))
  (Variables|Default|Setspline%20REF _returnvalue))

(fn ConstructionScript)