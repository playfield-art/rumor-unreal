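; Opinion actor that orbits the world center and can be summoned or dismissed by touch.
; It hides at BeginPlay, flies from center to its saved location on ShootOpinions, and reverses on backtomothership.
; Touch prints its tags, then either summons it to a fixed point, turning off glow, or shrinks it into the origin.
; Timelines drive all moves; after dismissal it regrows at center or saved location, depending on BP_MainWorld's IsPlaying.
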(event OnInputTouchBegin(Sphere)
  (params (FingerIndex :type ETouchIndex%20Enum :default "Touch1") (TouchedComponent :type Primitive%20Component%20Object%20Reference))
  ;[1 1 1] check to see which category it is in
  (for _array_element (Variables|Actor|GetTags)
    (Development|PrintString (Utilities|String|ToString(Name) _array_element) true true "(R=0.129912,G=1.000000,B=0.155829,A=1.000000)" 2e+02)
    (if (Variables|Default|GetisSummoned)
      (Variables|Default|SetgetOldScale (Transformation|GetActorScale3D))
      ;[1 1 1] back to mothership animation
      (bind _track (Timeline|Timeline_2 PlayFromStart)
        (:Update
          (Transformation|SetActorTransform (Math|Transform|MakeTransform (Math|Vector|Lerp(Vector) (Transformation|GetActorLocation) "0, 0, 0" _track) "0, 0, 0" (Math|Vector|Lerp(Vector) (Transformation|GetActorScale3D) "0, 0, 0" _track)))
          (Variables|Default|SetisSummoned false)
          ;[1 1 1] spawn new actor after delay from mothership to space
          (Utilities|FlowControl|Delay 5.0)
          (bind _returnvalue (Actor|GetActorOfClass "/Game/bluePrints/BP_MainWorld.BP_MainWorld_C"))
          (if (Variables|/Game/bluePrints/BP_MainWorld.BP_MainWorld_C|GetisPlaying _returnvalue)
            (bind _track_2 (Timeline|Timeline_4 PlayFromStart)
              (:Update
                (Transformation|SetActorTransform (Math|Transform|MakeTransform "0, 0,130.000000" "0, 0, 0" (Math|Vector|Lerp(Vector) "0, 0, 0" (Variables|Default|GetgetOldScale) _track_2)))))
            (else
              (bind _track_3 (Timeline|Timeline_3 PlayFromStart)
                (:Update
                  (Transformation|SetActorTransform (Math|Transform|MakeTransform (Math|Vector|Lerp(Vector) "0, 0, 0" (Variables|Default|GetnewLoc) _track_3) "0, 0, 0" (Math|Vector|Lerp(Vector) "0, 0, 0" (Variables|Default|GetgetOldScale) _track_3)))))))))
      (else
        ;[1 1 1] summon animation
        (bind _track_4 (Timeline|Timeline_1 PlayFromStart)
          (:Update
            (Transformation|SetActorLocation (Math|Vector|Lerp(Vector) (Transformation|GetActorLocation) "-1200.000000,-32.000000,330.000000" _track_4) false false)
            (Variables|Default|SetisSummoned true)
            ;[1 1 1] deactivate glow after delay
            (Utilities|FlowControl|Delay 0.2)
            (Components|Activation|Deactivate (Variables|Default|Getglow))))))))

(event Custom|startGlow
  (Components|Activation|Activate (Variables|Default|Getglow) false))

(event Custom|stopGlow
  (Components|Activation|Deactivate (Variables|Default|Getglow)))

(event Custom|ShootOpinions
  ;[1 1 1] set animation for opinions from center location to random location given by BP_opinionSpawn
  (bind _track (Timeline|Timeline_0 PlayFromStart)
    (:Update
      (Transformation|SetActorLocation (Math|Vector|Lerp(Vector) "0.000000, 0,130.000000" (Variables|Default|GetnewLoc) _track) false false))))

(event Custom|back%20to%20mothership
  ;[1 1 1] set animation for opinions from center location to random location given by BP_opinionSpawn
  (bind _track (Timeline|Timeline_0 Reverse)
    (:Update
      (Transformation|SetActorLocation (Math|Vector|Lerp(Vector) "0.000000, 0,130.000000" (Variables|Default|GetnewLoc) _track) false false))))

(event EventBeginPlay
  ;[1 1 1] set opinions out of sight in the beginning so it can spawn out of rumor
  (Variables|Default|SetnewLoc (Transformation|GetActorLocation))
  (Transformation|SetActorLocation "-1000000.000000, 0, 0" false false))

(event EventTick
  (params (DeltaSeconds :type Float%20%28single-precision%29))
  ;[1 1 1] rotate opinions around the x=0 y=0 z=0 axis
  (if (not (Variables|Default|GetisSummoned))
    (Transformation|SetActorLocation (+ (Math|Vector|RotateVectorAroundAxis (Transformation|GetActorLocation) (* DeltaSeconds (Variables|Default|GetSpeed)) (Variables|Default|GetAxis)) (Variables|Default|GetCenter%20Location)) false false)))

(fn ConstructionScript)