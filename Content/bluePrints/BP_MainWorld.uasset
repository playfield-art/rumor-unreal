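; Main world actor for the Rumor character, which wakes on click or touch by raising its Niagara tentacle point force and toggling a voice intro.
; The first tap also starts BP_splineFollower via DoOnce, while SleepMode and FirstPlayDone gate audio replays.
; Tick detects the audio ending, then grows BP_annemoon actors and shoots out BP_opinion actors, which later taps also toggle.
; Sphere click is a debug variant using a test sound.
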(event OnClicked(Sphere)
  (params (TouchedComponent :type Primitive%20Component%20Object%20Reference) (ButtonPressed :type Key%20Structure :default "None"))
  ;[1 1 1] Not neccisary, just to debug, so we can check with onclick function
  ;;[1 1 1] Wake up Rumor, set niagara tenticles  to 600 from point
  (Niagara|SetNiagaraVariable(Float) (Variables|Default|GetNiagara) "BPCallbackHandlerPointForce" 6e+02)
  ;;[1 1 1] check if animation just played, restet when game goes in sleepmode
  (if (Variables|Default|GetsleepMode)
    (Utilities|FlowControl|Delay 1.0)
    (Variables|Default|SetsleepMode false))
  ;;[1 1 1] check if audio is playing, play sound if not and keep reference, stop sound
  (if (Variables|Default|GetisPlaying)
    (Components|Activation|SetActive (stale _returnvalue) false true)
    (Variables|Default|SetisPlaying false)
    (else
      (bind _returnvalue (Audio|SpawnSound2D "/Game/Sound/rumor_test.rumor_test" 1.0 1.0 0.0 0))
      (Variables|Default|SetisPlaying true))))

(event EventBeginPlay
  ;[1 1 1] Set niagara tenticles to 50 velocity from point
  (Niagara|SetNiagaraVariable(Float) (Variables|Default|GetNiagara) "BPCallbackHandlerPointForce" 5e+01))

(event Collision|EventActorBeginOverlap
  (params (OtherActor :type Actor%20Object%20Reference)))

(event MouseInput|EventActorOnClicked
  (params (ButtonPressed :type Key%20Structure :default "None"))
  ;[1 1 1] Wake up Rumor, set niagara tenticles  to 600 from point
  (Niagara|SetNiagaraVariable(Float) (Variables|Default|GetNiagara) "BPCallbackHandlerPointForce" 6e+02)
  (Utilities|FlowControl|Sequence
    (:then_0
      ;[1 1 1] check if animation just played, reset it when game goes in sleepmode
      (if (Variables|Default|GetsleepMode)
        (Utilities|FlowControl|Delay 1.0)
        (Variables|Default|SetsleepMode false)
        ;[1 1 1] check if audio is playing, play sound if not and keep reference, stop sound
        (if (Variables|Default|GetisPlaying) :!label _label
          (Components|Activation|SetActive (stale _returnvalue) false true)
          (Variables|Default|SetisPlaying false)
          (else
            (bind _returnvalue (Audio|SpawnSound2D "/Game/Sound/vo-intro-rumor-personage_OTg2gZEC.vo-intro-rumor-personage_OTg2gZEC" 1.0 1.0 0.0 0))
            (Variables|Default|SetisPlaying true)
            (bind _outactors (Actor|GetAllActorsOfClass "/Game/bluePrints/BP_opinion.BP_opinion_C"))
            (for _array_element _outactors
              (Default|BacktoMothership _array_element)
              (Default|StopGlow _array_element)
              (Viewport|RemoveAllWidgets))))
        (elif (Variables|Default|GetfirstPlayDone)
          (goto _label))))
    (:then_1
      (Utilities|FlowControl|DoOnce false
        (:Completed
          (bind _returnvalue_2 (Actor|GetActorOfClass "/Game/bluePrints/BP_splineFollower.BP_splineFollower_C"))
          (Default|MoveObject _returnvalue_2))))
    (:then_2
      (if (Variables|Default|GetfirstPlayDone)
        (Utilities|FlowControl|Sequence
          (:then_0
            (bind _outactors_2 (Actor|GetAllActorsOfClass "/Game/bluePrints/BP_annemoon.BP_annemoon_C"))
            (for _array_element_2 _outactors_2
              (if (Variables|Default|GetisPlaying)
                (Default|Shrink _array_element_2)
                (else
                  (Default|StartGrow _array_element_2)))))
          (:then_1
            (bind _outactors_3 (Actor|GetAllActorsOfClass "/Game/bluePrints/BP_opinion.BP_opinion_C"))
            (for _array_element_3 _outactors_3
              (if (Variables|Default|GetisPlaying)
                (Default|BacktoMothership _array_element_3)
                (else
                  (Default|ShootOpinions _array_element_3))))))))))

(event EventTick
  (params (DeltaSeconds :type Float%20%28single-precision%29))
  ;[1 1 1] looks if first time audio played completely before moving on
  (if (Variables|Default|GetisPlaying)
    (if (not (Audio|Components|Audio|IsPlaying (stale MouseInput|EventActorOnClicked _returnvalue)))
      (Utilities|FlowControl|Sequence
        (:then_0
          (Variables|Default|SetisPlaying false)
          (Variables|Default|SetfirstPlayDone true))
        (:then_1
          (bind _outactors (Actor|GetAllActorsOfClass "/Game/bluePrints/BP_annemoon.BP_annemoon_C"))
          (for _array_element _outactors
            (Default|StartGrow _array_element)))
        (:then_2
          (bind _outactors_2 (Actor|GetAllActorsOfClass "/Game/bluePrints/BP_opinion.BP_opinion_C"))
          (for _array_element_2 _outactors_2
            (Default|ShootOpinions _array_element_2)))))))

(event EventActorOnInputTouchBegin
  (params (FingerIndex :type ETouchIndex%20Enum :default "Touch1"))
  ;[1 1 1] Wake up Rumor, set niagara tenticles  to 600 from point
  (Niagara|SetNiagaraVariable(Float) (Variables|Default|GetNiagara) "BPCallbackHandlerPointForce" 6e+02)
  (Utilities|FlowControl|Sequence
    (:then_0
      ;[1 1 1] check if animation just played, reset it when game goes in sleepmode
      (if (Variables|Default|GetsleepMode)
        (Utilities|FlowControl|Delay 1.0)
        (Variables|Default|SetsleepMode false)
        ;[1 1 1] check if audio is playing, play sound if not and keep reference, stop sound
        (if (Variables|Default|GetisPlaying) :!label _label
          (Components|Activation|SetActive (stale _returnvalue) false true)
          (Variables|Default|SetisPlaying false)
          (else
            (bind _returnvalue (Audio|SpawnSound2D "/Game/Sound/vo-intro-rumor-personage_OTg2gZEC.vo-intro-rumor-personage_OTg2gZEC" 1.0 1.0 0.0 0))
            (Variables|Default|SetisPlaying true)
            (bind _outactors (Actor|GetAllActorsOfClass "/Game/bluePrints/BP_opinion.BP_opinion_C"))
            (for _array_element _outactors
              (Default|BacktoMothership _array_element)
              (Default|StopGlow _array_element)
              (Viewport|RemoveAllWidgets))))
        (elif (Variables|Default|GetfirstPlayDone)
          (goto _label))))
    (:then_1
      (Utilities|FlowControl|DoOnce false
        (:Completed
          (bind _returnvalue_2 (Actor|GetActorOfClass "/Game/bluePrints/BP_splineFollower.BP_splineFollower_C"))
          (Default|MoveObject _returnvalue_2))))
    (:then_2
      (if (Variables|Default|GetfirstPlayDone)
        (Utilities|FlowControl|Sequence
          (:then_0
            (bind _outactors_2 (Actor|GetAllActorsOfClass "/Game/bluePrints/BP_annemoon.BP_annemoon_C"))
            (for _array_element_2 _outactors_2
              (if (Variables|Default|GetisPlaying)
                (Default|Shrink _array_element_2)
                (else
                  (Default|StartGrow _array_element_2)))))
          (:then_1
            (bind _outactors_3 (Actor|GetAllActorsOfClass "/Game/bluePrints/BP_opinion.BP_opinion_C"))
            (for _array_element_3 _outactors_3
              (if (Variables|Default|GetisPlaying)
                (Default|BacktoMothership _array_element_3)
                (else
                  (Default|ShootOpinions _array_element_3))))))))))

(fn ConstructionScript)