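; Spawner actor that creates BP_quote actors from JSON quote data when BP_MainWorld fires its create-quotes event, bound on BeginPlay.
; For each entry it reads the title in the current language and spawns one quote per "overall" item, tagged with that title and its index.
; AddLocationLogic places quotes around a ring by rotating an index-based radial offset about Z, adding seeded random position jitter and an unseeded random scale.
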(event Custom|CreateQuotes
  (params (quoteData :type Array%20of%20JSON%20Object%20Structures))
  (for _array_element quoteData
    (bind _returnvalue (Class|HTTPRequestClient|GetObjectfromJSONObject _array_element "title"))
    (bind _returnvalue_2 (Class|HTTPRequestClient|GetStringfromJSONObject _returnvalue (Class|KismetInternationalizationLibrary|GetCurrentLanguage)))
    (bind _returnvalue_3 (Class|HTTPRequestClient|GetObjectfromJSONObject _array_element "quotes"))
    (bind _returnvalue_4 (Class|HTTPRequestClient|GetObjectArrayfromJSONObject _returnvalue_3 "overall"))
    (Math|Integer|CompareInt (Utilities|Array|Length _returnvalue_4)
      (:>
        (for (_array_element_2 _array_index) _returnvalue_4
          (bind _maketransformvalue (CallFunction|AddLocationLogic _array_index))
          (bind _returnvalue_5 (Game|SpawnActorfromClass "/Game/bluePrints/BP_quote.BP_quote_C" _maketransformvalue "AdjustIfPossibleButAlwaysSpawn" 0 _returnvalue_2 0 _array_element_2 _array_index 0))
          (Variables|/Script/Engine.Actor|SetTags _returnvalue_5 (Utilities|Array|MakeArray (Utilities|String|StringToName _returnvalue_2))))))))

(event EventBeginPlay
  (bind _outactors (Actor|GetAllActorsOfClass "/Game/bluePrints/BP_MainWorld.BP_MainWorld_C"))
  (EventDispatchers|BindEventtoCreateQuotes (Utilities|Array|Get(acopy) _outactors) (delegate Custom|CreateQuotes)))

(fn ConstructionScript)

(fn AddLocationLogic
  (params (Index :type Integer))
  (bind _returnvalue (Math|Vector|MakeVector 0.0 0.0 1.0))
  (bind _returnvalue_2 (Math|Float|MakeLiteralFloat 3.6e+02))
  (bind _instances (Variables|Default|Getinstances))
  (bind _ring_width_ (Variables|Default|Getring%20width%20))
  (bind _instances_2 (Variables|Default|Getinstances))
  (bind _randomize_z_axis_position (Variables|Default|Getrandomize%20Z%20axis%20position))
  (bind _ring_width__2 (Variables|Default|Getring%20width%20))
  (bind _ring_radius (Variables|Default|Getring%20radius))
  (bind _transform_random (Variables|Default|Gettransform%20random))
  (bind _randomize_position (Variables|Default|Getrandomize%20position))
  (bind _returnvalue_3 (Math|Random|RandomFloatfromStream _transform_random))
  (bind _returnvalue_4 (Math|Random|RandomUnitVectorfromStream _transform_random))
  (bind _returnvalue_5 (/ Index _instances_2))
  (bind _returnvalue_6 (/ Index _instances))
  (bind _returnvalue_7 (* _returnvalue_4 _randomize_position))
  (bind _returnvalue_8 (- _returnvalue_5 0.5))
  (bind _returnvalue_9 (* _returnvalue_6 _returnvalue_2))
  (bind _returnvalue_10 (- _returnvalue_3 0.5))
  (bind _returnvalue_11 (* _returnvalue_8 _ring_width__2))
  (bind _returnvalue_12 (* _returnvalue_10 _randomize_z_axis_position _ring_width_))
  (bind _returnvalue_13 (+ _returnvalue_12 _returnvalue_7))
  (bind _returnvalue_14 (+ _returnvalue_11 _ring_radius))
  (bind _returnvalue_15 (Math|Vector|MakeVector 0.0 _returnvalue_14 6.5e+02))
  (bind _returnvalue_16 (+ _returnvalue_13 _returnvalue_15))
  (bind _returnvalue_17 (Math|Vector|RotateVectorAroundAxis _returnvalue_16 _returnvalue_9 _returnvalue))
  (return (Math|Transform|MakeTransform _returnvalue_17 "0, 0, 0" (Math|Conversions|ToVector(Float) (Math|Float|MapRangeClamped (Math|Random|RandomFloat) 0.0 1.0 0.2 0.4))) _returnvalue_17))