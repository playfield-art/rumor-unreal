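; BP_AmbientSoundMaster is an actor that switches the level's ambient surround sound by ID.
; On BeginPlay it finds BP_MainWorld and binds its play event to that actor's surround-sound event.
; The play event starts the indexed entry from AudioComponents, crossfading out any current sound over two seconds.
; The new component becomes CurrentSound after the delay, or immediately if nothing was playing.
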(event Custom|play
  (params (soundId :type Integer))
  (bind _audiocomponents (Variables|Default|GetaudioComponents))
  (bind _output (Utilities|Array|Get(acopy) _audiocomponents soundId))
  (bind _audiocomponent (Variables|/Script/Engine.AmbientSound|GetAudioComponent _output))
  (Utilities|IsValid (Variables|Default|GetcurrentSound)
    (:Is%20Valid
      (Audio|Components|Audio|Play _audiocomponent 0.0)
      (Audio|Components|Audio|FadeIn _audiocomponent 2.0 1.0 0.0 "Linear" :!class /Script/Engine.AudioComponent)
      (Audio|Components|Audio|FadeOut (Variables|Default|GetcurrentSound) 2.0 0.0 "Linear" :!class /Script/Engine.AudioComponent)
      (Utilities|FlowControl|Delay 2.0)
      (Variables|Default|SetcurrentSound _audiocomponent))
    (:Is%20Not%20Valid
      (Audio|Components|Audio|Play _audiocomponent 0.0)
      (Variables|Default|SetcurrentSound _audiocomponent))))

(event EventBeginPlay
  (bind _returnvalue (Actor|GetActorOfClass "/Game/bluePrints/BP_MainWorld.BP_MainWorld_C"))
  (EventDispatchers|BindEventtoPlaySurroundSound _returnvalue (delegate Custom|play)))

(fn ConstructionScript)