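; BP_annemoon is a touchable actor that highlights the BP_opinion actors linked to it by actor tags.
; Touching its Cylinder first stops the glow on every BP_opinion, then prints each of its own tags and starts the glow on BP_opinion actors carrying that tag.
; On BeginPlay it stores its scale and shrinks to zero, with nothing in this graph restoring it.
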(event OnInputTouchBegin(Cylinder)
  (params (FingerIndex :type ETouchIndex%20Enum :default "Touch1") (TouchedComponent :type Primitive%20Component%20Object%20Reference))
  (Utilities|FlowControl|Sequence
    (:then_0
      (bind _outactors (Actor|GetAllActorsOfClass "/Game/bluePrints/BP_opinion.BP_opinion_C"))
      (for _array_element _outactors
        (Default|StopGlow _array_element)))
    (:then_1
      (for _array_element_2 (Variables|Actor|GetTags)
        (Development|PrintString (Utilities|String|ToString(Name) _array_element_2))
        (bind _outactors_2 (Actor|GetAllActorswithTag _array_element_2))
        (for _array_element_3 _outactors_2
          (bind _asbp_opinion (Utilities|Casting|CastToBP_opinion _array_element_3))
          (Default|StartGlow _asbp_opinion))))))

(event Collision|EventActorBeginOverlap
  (params (OtherActor :type Actor%20Object%20Reference)))

(event EventTick
  (params (DeltaSeconds :type Float%20%28single-precision%29)))

(event EventBeginPlay
  (Variables|Default|Setscale (Transformation|GetActorScale3D))
  (Transformation|SetActorScale3D "0, 0, 0"))

(fn ConstructionScript)