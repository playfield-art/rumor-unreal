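; Highlighted child variant of an opinion actor that hides its Plane component while the actor is being summoned.
; After the parent Tick, it checks IsSummoned, scaling the Plane to zero after a short delay, or back to full size once summoning ends.
; Two DoOnce nodes reset each other so the scale is set only on state changes.
; An unconnected location-based visibility check remains in the graph.
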(event EventBeginPlay
  (|CallParentFunction) ; This node is disabled and will not be called.\nDrag off pins to build functionality.
)

(event Collision|EventActorBeginOverlap
  (params (OtherActor :type Actor%20Object%20Reference))
  (|CallParentFunction OtherActor) ; This node is disabled and will not be called.\nDrag off pins to build functionality.
)

(event EventTick
  (params (DeltaSeconds :type Float%20%28single-precision%29))
  (|CallParentFunction DeltaSeconds)
  (Utilities|FlowControl|Sequence
    (:then_0
      ;[1 1 1] hide plane if being summoned
      (if (Variables|Default|GetisSummoned)
        ;;[1 1 1] added do once to prevent continualy setting scale
        (Utilities|FlowControl|DoOnce false :!label _label
          (:Completed
            (Utilities|FlowControl|Delay 0.2)
            (Transformation|SetWorldScale3D (Variables|Default|GetPlane) "0, 0, 0")
            (goto _label_2 Reset)))
        (else
          (Utilities|FlowControl|DoOnce false :!label _label_2
            (:Completed
              (Transformation|SetWorldScale3D (Variables|Default|GetPlane) "1.000000,1.000000,1.000000")
              (goto _label Reset))))))))

(fn ConstructionScript
  (|CallParentFunction))