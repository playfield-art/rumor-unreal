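; BP_resetSpline is a clickable or touchable reset actor that replays the spline follower's line drawing.
; Its Reset component starts hidden on BeginPlay.
; Click or touch deactivates DrawLine on BP_splineFollower and hides Reset on every BP_resetSpline instance.
; A one-second Delay inside that loop then leads to calling MoveObject on the follower and reactivating DrawLine.
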(event EventBeginPlay
  (Rendering|SetVisibility (Variables|Default|Getreset) false false))

(event Collision|EventActorBeginOverlap
  (params (OtherActor :type Actor%20Object%20Reference)))

(event MouseInput|EventActorOnClicked
  (params (ButtonPressed :type Key%20Structure :default "None"))
  (bind _returnvalue (Actor|GetActorOfClass "/Game/bluePrints/BP_splineFollower.BP_splineFollower_C"))
  ;[1 1 1] deactivate line
  (Components|Activation|Deactivate (Variables|/Game/bluePrints/BP_splineFollower.BP_splineFollower_C|GetdrawLine _returnvalue))
  (bind _outactors (Actor|GetAllActorsOfClass "BP_resetSpline_C"))
  ;[1 1 1] de activate glow
  (for _array_element _outactors
    (Rendering|SetVisibility (Variables|BP_resetSpline_C|Getreset _array_element) false false)
    ;[1 1 1] start replay draw line
    (Utilities|FlowControl|Delay 1.0)
    (bind _returnvalue_2 (Actor|GetActorOfClass "/Game/bluePrints/BP_splineFollower.BP_splineFollower_C"))
    (Default|MoveObject _returnvalue_2)
    (Components|Activation|Activate (Variables|/Game/bluePrints/BP_splineFollower.BP_splineFollower_C|GetdrawLine _returnvalue) false)))

(event EventTick
  (params (DeltaSeconds :type Float%20%28single-precision%29)))

(event EventActorOnInputTouchBegin
  (params (FingerIndex :type ETouchIndex%20Enum :default "Touch1"))
  (bind _returnvalue (Actor|GetActorOfClass "/Game/bluePrints/BP_splineFollower.BP_splineFollower_C"))
  ;[1 1 1] deactivate line
  (Components|Activation|Deactivate (Variables|/Game/bluePrints/BP_splineFollower.BP_splineFollower_C|GetdrawLine _returnvalue))
  (bind _outactors (Actor|GetAllActorsOfClass "BP_resetSpline_C"))
  ;[1 1 1] de activate glow
  (for _array_element _outactors
    (Rendering|SetVisibility (Variables|BP_resetSpline_C|Getreset _array_element) false false)
    ;[1 1 1] start replay draw line
    (Utilities|FlowControl|Delay 1.0)
    (bind _returnvalue_2 (Actor|GetActorOfClass "/Game/bluePrints/BP_splineFollower.BP_splineFollower_C"))
    (Default|MoveObject _returnvalue_2)
    (Components|Activation|Activate (Variables|/Game/bluePrints/BP_splineFollower.BP_splineFollower_C|GetdrawLine _returnvalue) false)))

(fn ConstructionScript)