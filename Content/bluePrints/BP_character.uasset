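; Character Blueprint that lets the player tap interactable objects to summon an "opinion" for inspection, then release it.
; On Summon input, a cursor trace swaps the hit HISM instance for a BP_spawn child actor, re-adding an instance at a mirrored location.
; A timeline moves the actor to a reference point and opens a detail widget.
; Clicking a Spawn-tagged actor clears widgets, animates release, empties the child actor and resets the DoOnce gate.
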(event Custom|resetDoOnce
  (Utilities|FlowControl|DoOnce false) ; enters at Reset
)

(event Input|ActionEvents|InputActionSummon
  (params (Key :type Key%20Structure :default "None"))
  (bind _returnvalue (Game|GetPlayerController 0))
  (bind (_worldlocation _worlddirection) (Game|Player|ConvertMouseLocationToWorldSpace _returnvalue))
  (:Pressed
    ;[1 1 1] Make raytrace from touch to object
    (bind (_outhit _returnvalue_2) (Collision|LineTraceByChannel _worldlocation (+ _worldlocation (* _worlddirection 1e+04)) "TraceTypeQuery1" false 0 "None"))
    ;[1 1 1] check if we hit something
    (if _returnvalue_2
      ;[1 1 1] check if it hasn't got tag World and get hit info
      (if (Actor|ActorHasTag (.HitActor (Collision|BreakHitResult _outhit)) "Interactable")
        (Utilities|FlowControl|Sequence
          (:then_0
            (Utilities|FlowControl|Delay 0.1)
            (if (not (Variables|Default|GetviewingOpinion))
              ;[1 1 1] if start inspecting
              (Variables|Default|SetviewingOpinion true)
              ;;[1 1 1] set locations to animate between
              (Variables|Default|Setstart%20loc (Variables|/Script/Engine.SceneComponent|GetRelativeLocation (Variables|Default|GetChildOpinionActor)))
              (Variables|Default|Setend%20loc (Variables|/Script/Engine.SceneComponent|GetRelativeLocation (Variables|Default|GetOpinionReference)))
              ;;[1 1 1] animation
              (bind _track (Timeline|summonOpinion PlayFromStart)
                (:Update
                  (Transformation|SetRelativeLocation (Variables|Default|GetChildOpinionActor) (Math|Vector|Lerp(Vector) (Variables|Default|Getstart%20loc) (Variables|Default|Getend%20loc) _track) true false)
                  ;[1 1 1] add viewport widget (future image)
                  (Utilities|FlowControl|Delay 0.3)
                  (bind _returnvalue_3 (UserInterface|CreateWidget "/Game/detailPanel/WB_opinionDetail.WB_opinionDetail_C"))
                  (UserInterface|Viewport|AddtoViewport _returnvalue_3 0)))
              (else
                ;[1 1 1] Continue only when click on spawn element
                (if (Actor|ActorHasTag (.HitActor (Collision|BreakHitResult _outhit)) "Spawn")
                  ;[1 1 1] removes viewport image
                  (Viewport|RemoveAllWidgets)
                  (Utilities|FlowControl|Delay 0.1)
                  ;[1 1 1] if stop inspecting
                  (Variables|Default|SetviewingOpinion false)
                  (bind _track_2 (Timeline|releaseOpinion PlayFromStart)
                    (:Update
                      (Transformation|SetWorldLocation (Variables|Default|GetChildOpinionActor) (Math|Vector|Lerp(Vector) "-320.000000,-150.000000,-230.000000" "-60.000000,0.000000,-60.000000" _track_2) false false)
                      ;;[1 1 1] remove class from spawn to dissapeare
                      (Utilities|FlowControl|Delay 0.2)
                      (ChildActorComponent|SetChildActorClass (Variables|Default|GetChildOpinionActor) 0)
                      ;;[1 1 1] reset do once to view new opinion
                      (CallFunction|ResetDoOnce)))))))
          (:then_1
            (Utilities|FlowControl|DoOnce false
              (:Completed
                (ChildActorComponent|SetChildActorClass (Variables|Default|GetChildOpinionActor) "/Game/bluePrints/BP_spawn.BP_spawn_C")
                (Transformation|SetWorldLocation (Variables|Default|GetChildOpinionActor) (.Location (Collision|BreakHitResult _outhit)) false false)
                ;[1 1 1] Remove instance from HISMC to make it appear you summon it, then add instance at oposite location, not to loose instances
                (bind _ashierarchical_instanced_static_mesh_component (Utilities|Casting|CastToHierarchicalInstancedStaticMeshComponent (.HitComponent (Collision|BreakHitResult _outhit))))
                (Class|InstancedStaticMeshComponent|RemoveInstance _ashierarchical_instanced_static_mesh_component (.HitItem (Collision|BreakHitResult _outhit)))
                (Components|InstancedStaticMesh|AddInstance _ashierarchical_instanced_static_mesh_component (Math|Transform|MakeTransform (* (.Location (Collision|BreakHitResult _outhit)) "1.000000,-1.000000,-1.000000") "0, 0, 0" "0.120000,0.120000,0.120000") false)))))))))

(fn ConstructionScript)