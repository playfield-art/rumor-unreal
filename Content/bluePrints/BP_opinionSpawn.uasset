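; Spawner that fills the level at BeginPlay with ten tagged categories (cat1 to cat10) of BP_opinion actors arranged in a ring.
; Each category spawns a loop of opinions plus one highlighted child variant, placed using the category number as index.
; AddLocationLogic rotates each position around world Z by index, widening the radius across RingWidth into a spiral band.
; A random stream jitters position, while scale uses unseeded randomness.
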(event EventBeginPlay
  (Utilities|FlowControl|Sequence
    (:then_0
      (Utilities|FlowControl|Sequence
        (:then_0
          (for _index (range 0 (Variables|Default|Getinstances))
            (bind _maketransformvalue (CallFunction|AddLocationLogic _index))
            (bind _returnvalue (Game|SpawnActorfromClass "/Game/bluePrints/BP_opinion.BP_opinion_C" _maketransformvalue "AdjustIfPossibleButAlwaysSpawn" 0 0))
            (Variables|/Script/Engine.Actor|SetTags _returnvalue (Utilities|Array|MakeArray "cat1"))))
        (:then_1
          (bind _maketransformvalue_2 (CallFunction|AddLocationLogic 1))
          (bind _returnvalue_2 (Game|SpawnActorfromClass "/Game/bluePrints/BP_opinion_Child_Highlighted.BP_opinion_Child_Highlighted_C" _maketransformvalue_2 "AdjustIfPossibleButAlwaysSpawn" 0 0))
          (Variables|/Script/Engine.Actor|SetTags _returnvalue_2 (Utilities|Array|MakeArray "cat1")))))
    (:then_1
      (Utilities|FlowControl|Sequence
        (:then_0
          (for _index_2 (range 0 (Variables|Default|Getinstances))
            (bind _maketransformvalue_3 (CallFunction|AddLocationLogic _index_2))
            (bind _returnvalue_3 (Game|SpawnActorfromClass "/Game/bluePrints/BP_opinion.BP_opinion_C" _maketransformvalue_3 "AdjustIfPossibleButAlwaysSpawn" 0 0))
            (Variables|/Script/Engine.Actor|SetTags _returnvalue_3 (Utilities|Array|MakeArray "cat2"))))
        (:then_1
          (bind _maketransformvalue_4 (CallFunction|AddLocationLogic 2))
          (bind _returnvalue_4 (Game|SpawnActorfromClass "/Game/bluePrints/BP_opinion_Child_Highlighted.BP_opinion_Child_Highlighted_C" _maketransformvalue_4 "AdjustIfPossibleButAlwaysSpawn" 0 0))
          (Variables|/Script/Engine.Actor|SetTags _returnvalue_4 (Utilities|Array|MakeArray "cat2")))))
    (:then_2
      (Utilities|FlowControl|Sequence
        (:then_0
          (for _index_3 (range 0 (Variables|Default|Getinstances))
            (bind _maketransformvalue_5 (CallFunction|AddLocationLogic _index_3))
            (bind _returnvalue_5 (Game|SpawnActorfromClass "/Game/bluePrints/BP_opinion.BP_opinion_C" _maketransformvalue_5 "AdjustIfPossibleButAlwaysSpawn" 0 0))
            (Variables|/Script/Engine.Actor|SetTags _returnvalue_5 (Utilities|Array|MakeArray "cat3"))))
        (:then_1
          (bind _maketransformvalue_6 (CallFunction|AddLocationLogic 3))
          (bind _returnvalue_6 (Game|SpawnActorfromClass "/Game/bluePrints/BP_opinion_Child_Highlighted.BP_opinion_Child_Highlighted_C" _maketransformvalue_6 "AdjustIfPossibleButAlwaysSpawn" 0 0))
          (Variables|/Script/Engine.Actor|SetTags _returnvalue_6 (Utilities|Array|MakeArray "cat3")))))
    (:then_3
      (Utilities|FlowControl|Sequence
        (:then_0
          (for _index_4 (range 0 (Variables|Default|Getinstances))
            (bind _maketransformvalue_7 (CallFunction|AddLocationLogic _index_4))
            (bind _returnvalue_7 (Game|SpawnActorfromClass "/Game/bluePrints/BP_opinion.BP_opinion_C" _maketransformvalue_7 "AdjustIfPossibleButAlwaysSpawn" 0 0))
            (Variables|/Script/Engine.Actor|SetTags _returnvalue_7 (Utilities|Array|MakeArray "cat4"))))
        (:then_1
          (bind _maketransformvalue_8 (CallFunction|AddLocationLogic 4))
          (bind _returnvalue_8 (Game|SpawnActorfromClass "/Game/bluePrints/BP_opinion_Child_Highlighted.BP_opinion_Child_Highlighted_C" _maketransformvalue_8 "AdjustIfPossibleButAlwaysSpawn" 0 0))
          (Variables|/Script/Engine.Actor|SetTags _returnvalue_8 (Utilities|Array|MakeArray "cat4")))))
    (:then_4
      (Utilities|FlowControl|Sequence
        (:then_0
          (for _index_5 (range 0 (Variables|Default|Getinstances))
            (bind _maketransformvalue_9 (CallFunction|AddLocationLogic _index_5))
            (bind _returnvalue_9 (Game|SpawnActorfromClass "/Game/bluePrints/BP_opinion.BP_opinion_C" _maketransformvalue_9 "AdjustIfPossibleButAlwaysSpawn" 0 0))
            (Variables|/Script/Engine.Actor|SetTags _returnvalue_9 (Utilities|Array|MakeArray "cat5"))))
        (:then_1
          (bind _maketransformvalue_10 (CallFunction|AddLocationLogic 5))
          (bind _returnvalue_10 (Game|SpawnActorfromClass "/Game/bluePrints/BP_opinion_Child_Highlighted.BP_opinion_Child_Highlighted_C" _maketransformvalue_10 "AdjustIfPossibleButAlwaysSpawn" 0 0))
          (Variables|/Script/Engine.Actor|SetTags _returnvalue_10 (Utilities|Array|MakeArray "cat5")))))
    (:then_5
      (Utilities|FlowControl|Sequence
        (:then_0
          (for _index_6 (range 0 (Variables|Default|Getinstances))
            (bind _maketransformvalue_11 (CallFunction|AddLocationLogic _index_6))
            (bind _returnvalue_11 (Game|SpawnActorfromClass "/Game/bluePrints/BP_opinion.BP_opinion_C" _maketransformvalue_11 "AdjustIfPossibleButAlwaysSpawn" 0 0))
            (Variables|/Script/Engine.Actor|SetTags _returnvalue_11 (Utilities|Array|MakeArray "cat6"))))
        (:then_1
          (bind _maketransformvalue_12 (CallFunction|AddLocationLogic 6))
          (bind _returnvalue_12 (Game|SpawnActorfromClass "/Game/bluePrints/BP_opinion_Child_Highlighted.BP_opinion_Child_Highlighted_C" _maketransformvalue_12 "AdjustIfPossibleButAlwaysSpawn" 0 0))
          (Variables|/Script/Engine.Actor|SetTags _returnvalue_12 (Utilities|Array|MakeArray "cat6")))))
    (:then_6
      (Utilities|FlowControl|Sequence
        (:then_0
          (for _index_7 (range 0 (Variables|Default|Getinstances))
            (bind _maketransformvalue_13 (CallFunction|AddLocationLogic _index_7))
            (bind _returnvalue_13 (Game|SpawnActorfromClass "/Game/bluePrints/BP_opinion.BP_opinion_C" _maketransformvalue_13 "AdjustIfPossibleButAlwaysSpawn" 0 0))
            (Variables|/Script/Engine.Actor|SetTags _returnvalue_13 (Utilities|Array|MakeArray "cat7"))))
        (:then_1
          (bind _maketransformvalue_14 (CallFunction|AddLocationLogic 7))
          (bind _returnvalue_14 (Game|SpawnActorfromClass "/Game/bluePrints/BP_opinion_Child_Highlighted.BP_opinion_Child_Highlighted_C" _maketransformvalue_14 "AdjustIfPossibleButAlwaysSpawn" 0 0))
          (Variables|/Script/Engine.Actor|SetTags _returnvalue_14 (Utilities|Array|MakeArray "cat7")))))
    (:then_7
      (Utilities|FlowControl|Sequence
        (:then_0
          (for _index_8 (range 0 (Variables|Default|Getinstances))
            (bind _maketransformvalue_15 (CallFunction|AddLocationLogic _index_8))
            (bind _returnvalue_15 (Game|SpawnActorfromClass "/Game/bluePrints/BP_opinion.BP_opinion_C" _maketransformvalue_15 "AdjustIfPossibleButAlwaysSpawn" 0 0))
            (Variables|/Script/Engine.Actor|SetTags _returnvalue_15 (Utilities|Array|MakeArray "cat8"))))
        (:then_1
          (bind _maketransformvalue_16 (CallFunction|AddLocationLogic 8))
          (bind _returnvalue_16 (Game|SpawnActorfromClass "/Game/bluePrints/BP_opinion_Child_Highlighted.BP_opinion_Child_Highlighted_C" _maketransformvalue_16 "AdjustIfPossibleButAlwaysSpawn" 0 0))
          (Variables|/Script/Engine.Actor|SetTags _returnvalue_16 (Utilities|Array|MakeArray "cat8")))))
    (:then_8
      (Utilities|FlowControl|Sequence
        (:then_0
          (for _index_9 (range 0 (Variables|Default|Getinstances))
            (bind _maketransformvalue_17 (CallFunction|AddLocationLogic _index_9))
            (bind _returnvalue_17 (Game|SpawnActorfromClass "/Game/bluePrints/BP_opinion.BP_opinion_C" _maketransformvalue_17 "AdjustIfPossibleButAlwaysSpawn" 0 0))
            (Variables|/Script/Engine.Actor|SetTags _returnvalue_17 (Utilities|Array|MakeArray "cat9"))))
        (:then_1
          (bind _maketransformvalue_18 (CallFunction|AddLocationLogic 9))
          (bind _returnvalue_18 (Game|SpawnActorfromClass "/Game/bluePrints/BP_opinion_Child_Highlighted.BP_opinion_Child_Highlighted_C" _maketransformvalue_18 "AdjustIfPossibleButAlwaysSpawn" 0 0))
          (Variables|/Script/Engine.Actor|SetTags _returnvalue_18 (Utilities|Array|MakeArray "cat9")))))
    (:then_9
      (Utilities|FlowControl|Sequence
        (:then_0
          (for _index_10 (range 0 (Variables|Default|Getinstances))
            (bind _maketransformvalue_19 (CallFunction|AddLocationLogic _index_10))
            (bind _returnvalue_19 (Game|SpawnActorfromClass "/Game/bluePrints/BP_opinion.BP_opinion_C" _maketransformvalue_19 "AdjustIfPossibleButAlwaysSpawn" 0 0))
            (Variables|/Script/Engine.Actor|SetTags _returnvalue_19 (Utilities|Array|MakeArray "cat10"))))
        (:then_1
          (bind _maketransformvalue_20 (CallFunction|AddLocationLogic 10))
          (bind _returnvalue_20 (Game|SpawnActorfromClass "/Game/bluePrints/BP_opinion_Child_Highlighted.BP_opinion_Child_Highlighted_C" _maketransformvalue_20 "AdjustIfPossibleButAlwaysSpawn" 0 0))
          (Variables|/Script/Engine.Actor|SetTags _returnvalue_20 (Utilities|Array|MakeArray "cat10")))))))

(fn ConstructionScript)

(fn AddLocationLogic
  (params (Index :type Integer))
  (bind _returnvalue (Math|Vector|MakeVector 0.0 0.0 1.0))
  (bind _returnvalue_2 (Math|Float|MakeLiteralFloat 3.6e+02))
  (bind _ring_width_ (Variables|Default|Getring%20width%20))
  (bind _instances (Variables|Default|Getinstances))
  (bind _instances_2 (Variables|Default|Getinstances))
  (bind _randomize_z_axis_position (Variables|Default|Getrandomize%20Z%20axis%20position))
  (bind _ring_width__2 (Variables|Default|Getring%20width%20))
  (bind _ring_radius (Variables|Default|Getring%20radius))
  (bind _transform_random (Variables|Default|Gettransform%20random))
  (bind _randomize_position (Variables|Default|Getrandomize%20position))
  (bind _returnvalue_3 (Math|Random|RandomFloatfromStream _transform_random))
  (bind _returnvalue_4 (Math|Random|RandomUnitVectorfromStream _transform_random))
  (bind _returnvalue_5 (/ Index _instances))
  (bind _returnvalue_6 (/ Index _instances_2))
  (bind _returnvalue_7 (* _returnvalue_4 _randomize_position))
  (bind _returnvalue_8 (- _returnvalue_5 0.5))
  (bind _returnvalue_9 (* _returnvalue_6 _returnvalue_2))
  (bind _returnvalue_10 (- _returnvalue_3 0.5))
  (bind _returnvalue_11 (* _returnvalue_8 _ring_width__2))
  (bind _returnvalue_12 (* _returnvalue_10 _randomize_z_axis_position _ring_width_))
  (bind _returnvalue_13 (+ _returnvalue_12 _returnvalue_7))
  (bind _returnvalue_14 (+ _returnvalue_11 _ring_radius))
  (bind _returnvalue_15 (Math|Vector|MakeVector 0.0 _returnvalue_14 1e+02))
  (bind _returnvalue_16 (+ _returnvalue_13 _returnvalue_15))
  (bind _returnvalue_17 (Math|Vector|RotateVectorAroundAxis _returnvalue_16 _returnvalue_9 _returnvalue))
  (return (Math|Transform|MakeTransform _returnvalue_17 "0, 0, 0" (Math|Conversions|ToVector(Float) (Math|Float|MapRangeClamped (Math|Random|RandomFloat) 0.0 1.0 0.3 0.6))) _returnvalue_17))