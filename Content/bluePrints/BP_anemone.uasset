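; BP_anemone is a category marker actor that grows and shrinks vertically and can be touched or clicked to highlight related opinions.
; BeginPlay flattens its Category, Percentage and TopMark components; startGrow and shrink run a timeline forward or backward to scale their height and toggle the text.
; Selecting it stops glow on every BP_opinion, starts it on those matching its tags, opens a WB_cats widget and recolors its label as selected.
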(event OnClicked(Category)
  (params (TouchedComponent :type Primitive%20Component%20Object%20Reference) (ButtonPressed :type Key%20Structure :default "None"))
  (Utilities|FlowControl|Sequence
    (:then_0
      (bind _outactors (Actor|GetAllActorsOfClass "/Game/bluePrints/BP_opinion.BP_opinion_C"))
      (for _array_element _outactors
        (Default|StopGlow _array_element)))
    (:then_1
      (for _array_element_2 (Variables|Actor|GetTags)
        (Utilities|FlowControl|Sequence
          (:then_0
            (Development|PrintString (Utilities|String|ToString(Name) _array_element_2))
            (bind _outactors_2 (Actor|GetAllActorswithTag _array_element_2))
            (for _array_element_3 _outactors_2
              (bind _asbp_opinion (Utilities|Casting|CastToBP_opinion _array_element_3))
              (Default|StartGlow _asbp_opinion)))
          (:then_1
            (Viewport|RemoveAllWidgets)
            (bind _returnvalue (UserInterface|CreateWidget "/Game/detailPanel/WB_cats.WB_cats_C" (Game|GetPlayerController 0)))
            (bind _output_get (Variables|Default|SetUI _returnvalue))
            (UserInterface|Viewport|AddtoViewport _output_get 0)
            (Rendering|Components|TextRender|SetText (Variables|/Game/detailPanel/WB_cats.WB_cats_C|Gettitle (Variables|Default|GetUI)) (Variables|Default|GetUITitle))
            (Rendering|Components|TextRender|SetText (Variables|/Game/detailPanel/WB_cats.WB_cats_C|GetText (Variables|Default|GetUI)) (Variables|Default|GetUITitle))))))
    (:then_2
      (bind _outactors_3 (Actor|GetAllActorsOfClass "BP_anemone_C"))
      (for _array_element_4 _outactors_3
        (Rendering|Components|TextRender|SetTextRenderColor (Variables|BP_anemone_C|GetTextRender _array_element_4) (Variables|Default|Getoriginal%20color))))
    (:then_3
      (Utilities|FlowControl|Delay 0.1)
      (Rendering|Components|TextRender|SetTextRenderColor (Variables|Default|GetTextRender) (Variables|Default|Getclick%20color)))))

(event OnInputTouchBegin(Category)
  (params (FingerIndex :type ETouchIndex%20Enum :default "Touch1") (TouchedComponent :type Primitive%20Component%20Object%20Reference))
  (Utilities|FlowControl|Sequence
    (:then_0
      (bind _outactors (Actor|GetAllActorsOfClass "/Game/bluePrints/BP_opinion.BP_opinion_C"))
      (for _array_element _outactors
        (Default|StopGlow _array_element)))
    (:then_1
      (for _array_element_2 (Variables|Actor|GetTags)
        (Utilities|FlowControl|Sequence
          (:then_0
            (Development|PrintString (Utilities|String|ToString(Name) _array_element_2))
            (bind _outactors_2 (Actor|GetAllActorswithTag _array_element_2))
            (for _array_element_3 _outactors_2
              (bind _asbp_opinion (Utilities|Casting|CastToBP_opinion _array_element_3))
              (Default|StartGlow _asbp_opinion)))
          (:then_1
            (Viewport|RemoveAllWidgets)
            (bind _returnvalue (UserInterface|CreateWidget "/Game/detailPanel/WB_cats.WB_cats_C" (Game|GetPlayerController 0)))
            (bind _output_get (Variables|Default|SetUI _returnvalue))
            (UserInterface|Viewport|AddtoViewport _output_get 0)
            (Rendering|Components|TextRender|SetText (Variables|/Game/detailPanel/WB_cats.WB_cats_C|Gettitle (Variables|Default|GetUI)) (Variables|Default|GetUITitle))
            (Rendering|Components|TextRender|SetText (Variables|/Game/detailPanel/WB_cats.WB_cats_C|GetText (Variables|Default|GetUI)) (Variables|Default|GetUITitle))))))
    (:then_2
      (bind _outactors_3 (Actor|GetAllActorsOfClass "BP_anemone_C"))
      (for _array_element_4 _outactors_3
        (Rendering|Components|TextRender|SetTextRenderColor (Variables|BP_anemone_C|GetTextRender _array_element_4) (Variables|Default|Getoriginal%20color))))
    (:then_3
      (Utilities|FlowControl|Delay 0.1)
      (Rendering|Components|TextRender|SetTextRenderColor (Variables|Default|GetTextRender) (Variables|Default|Getclick%20color)))))

(event Custom|shrink
  (Utilities|FlowControl|Sequence
    (:then_0
      (bind _track (Timeline|Timeline_0 ReverseFromEnd)
        (:Update
          (Transformation|SetWorldScale3D (Variables|Default|GetCategory) (Math|Vector|MakeVector 0.3 0.3 (.z (Math|Vector|Lerp(Vector) "0.300000,0.300000, 0" (Variables|Default|Getscale%20category) _track))))
          (Transformation|SetWorldScale3D (Variables|Default|Gettop%20mark) (Math|Vector|MakeVector 0.3 0.3 (.z (Math|Vector|Lerp(Vector) "0.300000,0.300000, 0" (Variables|Default|Getscale%20top%20mark) _track))))
          (Transformation|SetWorldScale3D (Variables|Default|Getpercentage) (Math|Vector|MakeVector 0.3 0.3 (.z (Math|Vector|Lerp(Vector) "0.300000,0.300000, 0" (Variables|Default|Getscale%20percentage) _track)))))))
    (:then_1
      (Transformation|SetWorldScale3D (Variables|Default|GetTextRender) "0, 0, 0") ; Hide text
    )))

(event Custom|startGrow
  (Utilities|FlowControl|Sequence
    (:then_0
      ;[1 1 1] Show Text
      (Utilities|FlowControl|Delay 0.5)
      (Transformation|SetWorldScale3D (Variables|Default|GetTextRender) "0.500000,0.500000,1.000000"))
    (:then_1
      (bind _track (Timeline|Timeline_0 PlayFromStart)
        (:Update
          (Transformation|SetWorldScale3D (Variables|Default|GetCategory) (Math|Vector|MakeVector 0.3 0.3 (.z (Math|Vector|Lerp(Vector) "0.300000,0.300000, 0" (Variables|Default|Getscale%20category) _track))))
          (Transformation|SetWorldScale3D (Variables|Default|Gettop%20mark) (Math|Vector|MakeVector 0.3 0.3 (.z (Math|Vector|Lerp(Vector) "0.300000,0.300000, 0" (Variables|Default|Getscale%20top%20mark) _track))))
          (Transformation|SetWorldScale3D (Variables|Default|Getpercentage) (Math|Vector|MakeVector 0.3 0.3 (.z (Math|Vector|Lerp(Vector) "0.300000,0.300000, 0" (Variables|Default|Getscale%20percentage) _track)))))))))

(event EventBeginPlay
  (bind _percentage (Variables|Default|Getpercentage))
  (bind _category (Variables|Default|GetCategory))
  ;[1 1 1] set initial size to 0
  (Variables|Default|Setscale%20category (Transformation|GetWorldScale _category))
  (Transformation|SetWorldScale3D _category "0.300000,0.300000, 0")
  (Transformation|SetWorldScale3D (Variables|Default|GetTextRender) "0, 0, 0")
  (Variables|Default|Setscale%20percentage (Transformation|GetWorldScale _percentage))
  (Transformation|SetWorldScale3D _percentage "0.300000,0.300000, 0")
  (Transformation|SetWorldScale3D (Variables|Default|Gettop%20mark) "0.300000,0.300000, 0"))

(fn ConstructionScript)